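; SC_HearingSensor is a hearing sensor component that classifies listened targets into three levels by distance.
; Each tick it finds all actors of the listened classes and line traces to each on the Camera channel, optionally drawing debug lines.
; Hit distance against lower and upper bounds sets the level, stored with the impact point, or sensor location when out of range.
; Each target overwrites this data, so the last one wins.
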(event `self.ReceiveTick`
  (params (DeltaSeconds :type "Float (single-precision)"))
  (for _array_element (`self.ListenedTargets_Classes`)
    (bind _outactors (`GameplayStatics.GetAllActorsOfClass` _array_element))
    (for _array_element_2 _outactors
      (set `self.ActorCurrentlyListened` _array_element_2)
      (if (`self.ShowHearningLines?`)
        (set `self.HearningLines_DrawType` "ForOneFrame")
        (else
          (set `self.HearningLines_DrawType` "None")))
      (bind _outhit (`KismetSystemLibrary.LineTraceSingle` :`Start` (`self.K2_GetComponentLocation` self) :`End` (+ (`Actor.K2_GetActorLocation` (`self.ActorCurrentlyListened`)) (`self.TargetDisplacementValue`)) :`TraceChannel` "TraceTypeQuery2" :`DrawDebugType` (`self.HearningLines_DrawType`)))
      (set `self.ActorCurrentlyListened_Distance` (`.Distance` (`GameplayStatics.BreakHitResult` _outhit)))
      (set `self.ActorCurrentlyListened_SoundLocation` (`.ImpactPoint` (`GameplayStatics.BreakHitResult` _outhit)))
      (if (<= (`self.ActorCurrentlyListened_Distance`) (`.Value` (break `FloatRangeBound` (`.UpperBound` (break `FloatRange` (`self.ListenedTargets_Values`))))))
        (if (<= (`self.ActorCurrentlyListened_Distance`) (`.Value` (break `FloatRangeBound` (break `FloatRange` (`self.ListenedTargets_Values`)))))
          (set `self.HearingOwner_HearingData` (make `/Game/Blueprints/F_HearingData` "NewEnumerator2" (`self.ActorCurrentlyListened_SoundLocation`)))
          (else
            (set `self.HearingOwner_HearingData` (make `/Game/Blueprints/F_HearingData` "NewEnumerator1" (`self.ActorCurrentlyListened_SoundLocation`)))))
        (else
          (set `self.HearingOwner_HearingData` (make `/Game/Blueprints/F_HearingData` "NewEnumerator0" (`self.K2_GetComponentLocation` self))))))))