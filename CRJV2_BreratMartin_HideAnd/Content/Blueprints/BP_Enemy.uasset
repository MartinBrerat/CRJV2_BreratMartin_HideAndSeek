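; BP_Enemy is an enemy that reacts to noises reported by its SCHearingSensor.
; Each Tick reads the sensor's hearing state and stores the sound location for distant or close noises.
; The distant reaction turns the enemy toward the sound on yaw only.
; The close reaction runs AIMoveTo to that location behind a DoOnce gate, which resets only when the move succeeds.
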(event `self.ReceiveTick`
  (params (DeltaSeconds :type "Float (single-precision)"))
  (bind (_hearingowner_hearingdata_hearingstate _hearingowner_hearingdata_soundlocation) (break `/Game/Blueprints/F_HearingData` (`/Game/Blueprints/SC_HearingSensor.HearingOwner_HearingData` (`self.SC_HearingSensor`))))
  (switch `/Game/Blueprints/E_HearingStates` _hearingowner_hearingdata_hearingstate
    (:`NewEnumerator1`
      (set `self.AI_SoundHeard_Location` _hearingowner_hearingdata_soundlocation)
      (`self.Hearing_Distant`))
    (:`NewEnumerator2`
      (set `self.AI_SoundHeard_Location` _hearingowner_hearingdata_soundlocation)
      (`self.Hearing_Close`))))

(event `Hearing_Distant`
  (bind (_returnvalue_roll _returnvalue_pitch _returnvalue_yaw) (`KismetMathLibrary.BreakRotator` (`KismetMathLibrary.FindLookAtRotation` (`self.K2_GetActorLocation` self) (`self.AI_SoundHeard_Location`))))
  (`self.K2_SetActorRotation` (`KismetMathLibrary.MakeRotator` 0.0 0.0 _returnvalue_yaw)))

(event `Hearing_Close`
  (`/Engine/EditorBlueprintResources/StandardMacros.DoOnce` false :!label _label
    (:`Completed`
      (`|AIMoveTo` self (`self.AI_SoundHeard_Location`) null
        (:`OnSuccess`
          (`self.Reset DoOnce`))))))

(event `Reset DoOnce`
  (goto _label :!via `Reset`))

(fn `UserConstructionScript`)