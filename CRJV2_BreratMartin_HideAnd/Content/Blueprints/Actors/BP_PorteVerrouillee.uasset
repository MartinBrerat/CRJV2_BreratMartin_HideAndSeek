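; BP_PorteVerrouillee is a locked door actor that the player can operate only while holding a key.
; PlayerMessage stores look distance and interaction input, then, within range, routes them through condition checks to a currently empty shader event and to DirectInteraction.
; DirectInteraction checks the character's KeyPossessed flag, printing a French no-key message or alternating a timeline forward and backward via FlipFlop to rotate the door.
; The key flag clears when the timeline finishes.
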(event `/Game/Blueprints/Tools/BPI_Player.PlayerMessage`
  (params (Distance :type "Float (single-precision)") (`Interaction?` :type Boolean) (`KeyPossessed?` :type Boolean))
  (set `self.IV_Distance` Distance)
  (set `self.IV_Interaction?` `Interaction?`)
  (`|ExecutionSequence`
    (:`then_0`
      (if (<= (`self.IV_Distance`) (`self.SelfLookedAtDistance`))
        (if (`self.IsActorDisplayingShaderOnInteraction?`)
          (`self.Play Interaction Shader`))
        (if (`self.IV_Interaction?`)
          (if (`self.IsActorReactingToInteraction?`)
            (`self.Direct Interaction`)))))))

(event `Play Interaction Shader`)

(event `Direct Interaction`
  (bind _door_door (`self.Door_Door`))
  (bind _asbp_first_person_character_original (cast `/Game/Blueprints/Pawns/BP_First_Person_Character_original` (`GameplayStatics.GetPlayerPawn` 0)))
  (if (`/Game/Blueprints/Pawns/BP_First_Person_Character_original.Key_Possessed` _asbp_first_person_character_original)
    (`/Engine/EditorBlueprintResources/StandardMacros.FlipFlop`
      (:`A`
        (bind (_direction _newtrack_1) (`Timeline|Ouverture_Porte` :!via `PlayFromStart` :!label _label)
          (:`Update`
            (`SceneComponent.K2_SetRelativeRotation` _door_door (`KismetMathLibrary.RLerp` (`SceneComponent.RelativeRotation` _door_door) (struct :`Yaw` 90.0) _newtrack_1) false false))
          (:`Finished`
            (set `/Game/Blueprints/Pawns/BP_First_Person_Character_original.Key_Possessed` false _asbp_first_person_character_original))))
      (:`B`
        (goto _label :!via `ReverseFromEnd`)))
    (else
      (`KismetSystemLibrary.PrintString` "Tu n'a pas de clé"))))

(fn `UserConstructionScript`)