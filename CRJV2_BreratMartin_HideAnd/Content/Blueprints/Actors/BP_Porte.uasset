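; BP_Porte is a door actor that the player interacts with by looking at it within range.
; PlayerMessage stores distance and input, then gates the empty shader hook and DirectInteraction by range and per-actor flags.
; DirectInteraction flip-flops the Ouverture_Porte timeline forward and backward to drive DoorDoor's rotation.
; Each update lerps from the current rotation toward a fixed 90-degree target, so reversing never restores the closed pose.
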(event `/Game/Blueprints/Tools/BPI_Player.PlayerMessage`
  (params (Distance :type "Float (single-precision)") (`Interaction?` :type Boolean) (`KeyPossessed?` :type Boolean))
  (set `self.IV_Distance` Distance)
  (set `self.IV_Interaction?` `Interaction?`)
  (`|ExecutionSequence`
    (:`then_0`
      (if (<= (`self.IV_Distance`) (`self.SelfLookedAtDistance`))
        (if (`self.IsActorDisplayingShaderOnInteraction?`)
          (`self.Play Interaction Shader`))
        (if (`self.IV_Interaction?`)
          (if (`self.IsActorReactingToInteraction?`)
            (`self.Direct Interaction`)))))))

(event `Play Interaction Shader`)

(event `Direct Interaction`
  (bind _door_door (`self.Door_Door`))
  (cast `/Game/FirstPersonBP/Blueprints/FirstPersonCharacter` (`GameplayStatics.GetPlayerPawn` 0))
  (`/Engine/EditorBlueprintResources/StandardMacros.FlipFlop`
    (:`A`
      (bind (_direction _newtrack_1) (`Timeline|Ouverture_Porte` :!via `PlayFromStart` :!label _label)
        (:`Update`
          (`SceneComponent.K2_SetRelativeRotation` _door_door (`KismetMathLibrary.RLerp` (`SceneComponent.RelativeRotation` _door_door) (struct :`Yaw` 90.0) _newtrack_1) false false))))
    (:`B`
      (goto _label :!via `ReverseFromEnd`))))

(fn `UserConstructionScript`)