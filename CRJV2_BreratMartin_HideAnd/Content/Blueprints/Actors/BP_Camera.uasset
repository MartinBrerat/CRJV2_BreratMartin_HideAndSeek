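; BP_Camera is a camera actor that signals an alert when the first-person player character enters its detection box.
; Box begin and end overlaps, filtered by a cast to FirstPersonCharacter, call Alert and Unalert.
; Alert turns the SpotLight red and Unalert returns it to white, both printing the same on-screen siren text as placeholder feedback.
; An unconnected timeline is never run.
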(event `self.Box.OnComponentBeginOverlap`
  (params (OverlappedComponent :type "PrimitiveComponent Object Reference") (OtherActor :type "Actor Object Reference") (OtherComp :type "PrimitiveComponent Object Reference") (OtherBodyIndex :type Integer) (bFromSweep :type Boolean) (SweepResult :type "HitResult Structure (by ref)"))
  ;[1 1 1] Camera
  (cast `/Game/FirstPersonBP/Blueprints/FirstPersonCharacter` OtherActor)
  (`self.Alert`))

(event `self.Box.OnComponentEndOverlap`
  (params (OverlappedComponent :type "PrimitiveComponent Object Reference") (OtherActor :type "Actor Object Reference") (OtherComp :type "PrimitiveComponent Object Reference") (OtherBodyIndex :type Integer))
  ;[1 1 1] Camera
  (cast `/Game/FirstPersonBP/Blueprints/FirstPersonCharacter` OtherActor)
  (`self.Unalert`))

(fn `Alert`
  (`LightComponent.SetLightColor` (`self.SpotLight`) (struct :`R` 1.0 :`G` 0.018722 :`A` 1.0) true)
  (`KismetSystemLibrary.PrintString` "BEEDOBEEDOBEEDOBEEDOBEEDOBEEDOBEEDOBEEDOBEEDOBEEDOBEEDOBEEDO"))

(fn `Unalert`
  (`LightComponent.SetLightColor` (`self.SpotLight`) (struct :`R` 1.0 :`G` 1.0 :`B` 1.0 :`A` 1.0) true)
  (`KismetSystemLibrary.PrintString` "BEEDOBEEDOBEEDOBEEDOBEEDOBEEDOBEEDOBEEDOBEEDOBEEDOBEEDOBEEDO"))

(fn `UserConstructionScript`)