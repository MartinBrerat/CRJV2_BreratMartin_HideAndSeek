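; BP_Trousseau is a key pickup actor that sets KeyPossessed on the FirstPersonCharacter and destroys itself when taken.
; PlayerMessage calls its parent, stores distance and interaction, then conditionally plays an interaction shader if SelfLookedAtDistance is non-negative.
; Within that check, an interaction conditionally fires DirectInteraction, then repeats the key grant and destroy inline.
; A separate Grab function duplicates DirectInteraction's debug print and pickup logic.
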(event `/Game/Blueprints/Tools/BPI_Player.PlayerMessage`
  (params (Distance :type "Float (single-precision)") (`Interaction?` :type Boolean) (`KeyPossessed?` :type Boolean))
  (`parent.PlayerMessage` Distance `Interaction?` false)
  (set `self.IV_Distance` Distance)
  (set `self.IV_Interaction?` `Interaction?`)
  (`|ExecutionSequence`
    (:`then_0`
      (if (<= 0.0 (`self.SelfLookedAtDistance`))
        (if (`self.IsActorDisplayingShaderOnInteraction?`)
          (`self.Play Interaction Shader`))
        (if (`self.IV_Interaction?`)
          (if (`self.IsActorReactingToInteraction?`)
            (`self.Direct_Interaction`))
          (bind _asfirst_person_character (cast `/Game/FirstPersonBP/Blueprints/FirstPersonCharacter` (`GameplayStatics.GetPlayerPawn` 0)))
          (set `/Game/FirstPersonBP/Blueprints/FirstPersonCharacter.KeyPossessed` true _asfirst_person_character)
          (`self.K2_DestroyActor`))))))

(event `Direct_Interaction`)

(event `self.Direct Interaction`
  (`KismetSystemLibrary.PrintString` "Wooooho")
  (bind _asfirst_person_character (cast `/Game/FirstPersonBP/Blueprints/FirstPersonCharacter` (`GameplayStatics.GetPlayerPawn` 0)))
  (set `/Game/FirstPersonBP/Blueprints/FirstPersonCharacter.KeyPossessed` true _asfirst_person_character)
  (`self.K2_DestroyActor`))

(fn `Grab`
  (`KismetSystemLibrary.PrintString` "Wooooho")
  (bind _asfirst_person_character (cast `/Game/FirstPersonBP/Blueprints/FirstPersonCharacter` (`GameplayStatics.GetPlayerPawn` 0)))
  (set `/Game/FirstPersonBP/Blueprints/FirstPersonCharacter.KeyPossessed` true _asfirst_person_character)
  (`self.K2_DestroyActor`))

(fn `UserConstructionScript`
  (`parent.UserConstructionScript`))