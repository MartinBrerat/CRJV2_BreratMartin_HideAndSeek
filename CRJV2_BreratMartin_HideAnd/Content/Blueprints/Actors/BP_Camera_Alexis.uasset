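; BP_Camera_Alexis is a camera actor that raises an alert when the player character enters its detection Box.
; On begin overlap, Alerte turns light E red and calls PlayerSpotedMessage with the Box's world location.
; On end overlap, FinAlerte turns the light white, but only if the Box still reports overlapping the player character.
; Detection is purely overlap-driven, with no Tick logic or line-of-sight check.
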(event `self.Box.OnComponentBeginOverlap`
  (params (OverlappedComponent :type "PrimitiveComponent Object Reference") (OtherActor :type "Actor Object Reference") (OtherComp :type "PrimitiveComponent Object Reference") (OtherBodyIndex :type Integer) (bFromSweep :type Boolean) (SweepResult :type "HitResult Structure (by ref)"))
  (if (`PrimitiveComponent.IsOverlappingActor` (`self.Box`) (`GameplayStatics.GetPlayerCharacter` 0))
    (`self.Alerte`)))

(event `self.Box.OnComponentEndOverlap`
  (params (OverlappedComponent :type "PrimitiveComponent Object Reference") (OtherActor :type "Actor Object Reference") (OtherComp :type "PrimitiveComponent Object Reference") (OtherBodyIndex :type Integer))
  (if (`PrimitiveComponent.IsOverlappingActor` (`self.Box`) (`GameplayStatics.GetPlayerCharacter` 0))
    (`self.FinAlerte`)))

(fn `Alerte`
  (`LightComponent.SetLightColor` (`self.e`) (struct :`R` 1.0 :`A` 1.0) true)
  (message `/Game/Blueprints/Tools/BPI_Player.PlayerSpoted` self (`SceneComponent.K2_GetComponentLocation` (`self.Box`))))

(fn `FinAlerte`
  (`LightComponent.SetLightColor` (`self.e`) (struct :`R` 1.0 :`G` 1.0 :`B` 1.0 :`A` 1.0) true))

(fn `UserConstructionScript`)