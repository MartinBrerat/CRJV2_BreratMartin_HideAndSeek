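; BP_InteractiveActor is an actor that responds to player look-at and interaction messages, apparently as a base for interactive objects.
; PlayerMessage stores the incoming distance and interaction flag, then checks the distance against SelfLookedAtDistance.
; Within range, per-actor booleans gate PlayInteractionShader and, when interaction is requested, DirectInteraction.
; Both response events are placeholders that only print strings.
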(event `/Game/Blueprints/Tools/BPI_Player.PlayerMessage`
  (params (Distance :type "Float (single-precision)") (`Interaction?` :type Boolean))
  (set `self.IV_Distance` Distance)
  (set `self.IV_Interaction?` `Interaction?`)
  (`|ExecutionSequence`
    (:`then_0`
      (if (<= (`self.IV_Distance`) (`self.SelfLookedAtDistance`))
        (if (`self.IsActorDisplayingShaderOnInteraction?`)
          (`self.Play Interaction Shader`))
        (if (`self.IV_Interaction?`)
          (if (`self.IsActorReactingToInteraction?`)
            (`self.Direct Interaction`)))))))

(event `Play Interaction Shader`
  (`KismetSystemLibrary.PrintString` "HERE WILL BE PLAYED INTERACTION SHADER"))

(event `Direct Interaction`
  (`KismetSystemLibrary.PrintString` "HERE WILL BE PLAYED DIRECT INTERACTION BEHAVIOUR"))

(fn `UserConstructionScript`)