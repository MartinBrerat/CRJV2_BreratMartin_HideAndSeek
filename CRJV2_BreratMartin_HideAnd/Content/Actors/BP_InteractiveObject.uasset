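; BP_InteractiveObject is an actor that reacts to the player looking at it or interacting with it.
; PlayerMessage stores distance and interaction, then gates shader and interaction events through macros using per-actor flags and a SelfLookedAtDistance check.
; DirectInteraction assigns its StaticMesh to FirstPersonCharacter's CurrentMesh, or prints a French message if one is already held.
; PlayInteractionShader is empty, and the physics-off, GripPoint attachment logic is disconnected.
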(event `/Game/Blueprints/Misc/BPI_Player.PlayerMessage`
  (params (Distance :type "Float (single-precision)") (`Interaction?` :type Boolean))
  (set `self.IV_Distance` Distance)
  (set `self.IV_Interaction?` `Interaction?`)
  (`|ExecutionSequence`
    (:`then_0`
      (if (<= 0.0 (`self.SelfLookedAtDistance`))
        (if (`self.IsActorDisplayingShaderOnInteraction?`)
          (`self.Play Interaction Shader`))
        (if (`self.IV_Interaction?`)
          (if (`self.IsActorReactingToInteraction?`)
            (`self.Direct Interaction`)))))))

(event `Play Interaction Shader`)

(event `Direct Interaction`
  (bind _asfirst_person_character (cast `/Game/FirstPersonBP/Blueprints/FirstPersonCharacter` (`GameplayStatics.GetPlayerPawn` 0)))
  (if (!= (`/Game/FirstPersonBP/Blueprints/FirstPersonCharacter.CurrentMesh` _asfirst_person_character) null)
    (`KismetSystemLibrary.PrintString` "Tu tient déjà un objet")
    (else
      (set `/Game/FirstPersonBP/Blueprints/FirstPersonCharacter.CurrentMesh` (`self.StaticMesh`) _asfirst_person_character))))

(fn `UserConstructionScript`)