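; Security camera actor that detects the player through a Box trigger and signals with its SpotLight.
; Box begin and end overlaps with FirstPersonCharacter call Alert and Unalerted, switching the light between red and white and printing a status message.
; Tick resets the Box's relative rotation to zero every frame.
; A RotateCamera call and two alternative detection checks remain unconnected.
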(event `self.ReceiveTick`
  (params (DeltaSeconds :type "Float (single-precision)"))
  (`SceneComponent.K2_SetRelativeRotation` :`self` (`self.Box`)))

(event `self.Box.OnComponentBeginOverlap`
  (params (OverlappedComponent :type "PrimitiveComponent Object Reference") (OtherActor :type "Actor Object Reference") (OtherComp :type "PrimitiveComponent Object Reference") (OtherBodyIndex :type Integer) (bFromSweep :type Boolean) (SweepResult :type "HitResult Structure (by ref)"))
  ;[1 1 1] Méthode Corentin
  (cast `/Game/FirstPersonBP/Blueprints/FirstPersonCharacter` OtherActor)
  (`self.Alert`))

(event `self.Box.OnComponentEndOverlap`
  (params (OverlappedComponent :type "PrimitiveComponent Object Reference") (OtherActor :type "Actor Object Reference") (OtherComp :type "PrimitiveComponent Object Reference") (OtherBodyIndex :type Integer))
  (cast `/Game/FirstPersonBP/Blueprints/FirstPersonCharacter` OtherActor)
  (`self.Unalerted`))

(fn `Alert`
  (`LightComponent.SetLightColor` (`self.SpotLight`) (struct :`R` 1.0 :`B` 0.01736 :`A` 1.0) true)
  (`KismetSystemLibrary.PrintString` "WEEWOOWEEWOOWEEWOOWEEWOOWEEWOOWEEWOO"))

(fn `Unalerted`
  (`LightComponent.SetLightColor` (`self.SpotLight`) (struct :`R` 1.0 :`G` 1.0 :`B` 1.0 :`A` 1.0) true)
  (`KismetSystemLibrary.PrintString` "Nothing to report "))

(fn `UserConstructionScript`)